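; BP_Ribbon is a self-cleaning Niagara effect actor, named as a ribbon effect.
; On BeginPlay it activates its main NiagaraComponent and six additional Niagara components together, without resetting them.
; It then enables destroy-on-system-finish, so no manual cleanup logic is needed.
; Tick and the construction script are empty.
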(event `self.ReceiveBeginPlay`
  (`ActorComponent.Activate` (`self.NiagaraComponent`) false)
  (`ActorComponent.Activate` (`self.Niagara3`) false)
  (`ActorComponent.Activate` (`self.Niagara`) false)
  (`ActorComponent.Activate` (`self.Niagara1`) false)
  (`ActorComponent.Activate` (`self.Niagara2`) false)
  (`ActorComponent.Activate` (`self.Niagara4`) false)
  (`ActorComponent.Activate` (`self.Niagara5`) false)
  (`self.SetDestroyOnSystemFinish` true))

(event `self.ReceiveTick`
  (params (DeltaSeconds :type "Float (single-precision)")))

(fn `UserConstructionScript`)